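; Obstacle spawner for the Endless Runner Creator's vertical runner mode, placing obstacles alternately at left and right X positions.
; It extends a parent spawner's enable and spawn functions, repositioning any valid actor the parent provides at the spawner's Y and Z.
; Each obstacle gets a random Z scale, and the side flips after every placement, starting on the left.
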(event EventBeginPlay
  (|CallParentFunction)
  ;[0 0 0] Default initial side to spawn items to the left.
  (Variables|SpawnerOptions|SetbSpawningRight false))

(fn ConstructionScript
  (|CallParentFunction))

(fn EnableActor
  ;[0 0 0] Make sure to call parent implementation first to see if there's an obstacle available to enable.
  (|CallParentFunction)
  ;[0 0 0] If parent class was able to enable an obstacle then "CurrentObstacle" should be valid.
  (Utilities|IsValid (Variables|Default|GetCurrentActor)
    (:Is%20Valid
      ;[0 0 0] If "CurrentObstacle" is valid then set its location and scale
      (CallFunction|SetCurrentObstacleLocationScale))))

(fn TrySpawnNewActor
  ;[0 0 0] Make sure to call parent implementation first to see if there's an obstacle available to spawn
  (|CallParentFunction)
  ;[0 0 0] If parent class was able to spawn an obstacle then "CurrentObstacle" should be valid.
  (Utilities|IsValid (Variables|Default|GetCurrentActor)
    (:Is%20Valid
      ;[0 0 0] If "CurrentObstacle" is valid then set its location and scale
      (CallFunction|SetCurrentObstacleLocationScale))))

(fn SetCurrentObstacleLocationScale
  (bind _returnvalue (Transformation|GetActorLocation))
  (bind _returnvalue_2 (Transformation|GetActorLocation))
  (Transformation|SetActorLocation (Variables|Default|GetCurrentActor) (Math|Vector|SelectVector (Math|Vector|MakeVector (Variables|SpawnerOptions|GetRightSpawnPosition) (.y _returnvalue_2) (.z _returnvalue_2)) (Math|Vector|MakeVector (Variables|SpawnerOptions|GetLeftSpawnPosition) (.y _returnvalue) (.z _returnvalue)) (Variables|SpawnerOptions|GetbSpawningRight)) false false)
  (Transformation|SetActorScale3D (Variables|Default|GetCurrentActor) (Math|Vector|MakeVector 0.5 1.0 (Math|Random|RandomFloatinRange 0.2 1.0)))
  (Variables|SpawnerOptions|SetbSpawningRight (not (Variables|SpawnerOptions|GetbSpawningRight))))