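; Player for a vertical endless runner that jumps between two walls on touch, starting on the right wall.
; A single MoveAnim timeline drives location, pitch and a squash scale relative to the stored start location, playing forward to move left and in reverse to move right.
; A touch plays a whoosh, then starts a move if CanMove allows, and the timeline's finish flips the wall side and clears the moving flag.
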(event Custom|MoveLeft
  (bind (_direction _pitch _scaleanimation _ratio) (Timeline|MoveAnim PlayFromStart)
    (:Update
      ;[0 0 0] Update the player location and rotation to travel to the opposite wall
      (Transformation|SetActorLocationAndRotation (+ (Variables|Default|GetStartLocation) (Math|Vector|MakeVector (* (Variables|Default|GetDistanceBetweenWalls) (.x _ratio)) (.y _ratio) (* (.z _ratio) (Variables|Default|GetJumpHeight)))) (Math|Rotator|MakeRotator 0.0 _pitch 0.0))
      ;[0 0 0] Apply a scale update as a simple squash animation.
      (Transformation|SetActorScale3D (Math|Vector|MakeVector (Math|Float|Lerp 1.0 0.5 _scaleanimation) 0.0 (Math|Float|Lerp 1.0 0.5 _scaleanimation))))
    (:Finished
      ;[0 0 0] Track the current side the player is on.
      (Variables|Default|SetbOnRightWall (not (Variables|Default|GetbOnRightWall)))
      ;[0 0 0] Reset bMoving so that the player is able to jump again.
      (Variables|Default|SetbMoving false))))

(event Custom|MoveRight
  (bind (_direction _pitch _scaleanimation _ratio) (Timeline|MoveAnim ReverseFromEnd)
    (:Update
      ;[0 0 0] Update the player location and rotation to travel to the opposite wall
      (Transformation|SetActorLocationAndRotation (+ (Variables|Default|GetStartLocation) (Math|Vector|MakeVector (* (Variables|Default|GetDistanceBetweenWalls) (.x _ratio)) (.y _ratio) (* (.z _ratio) (Variables|Default|GetJumpHeight)))) (Math|Rotator|MakeRotator 0.0 _pitch 0.0))
      ;[0 0 0] Apply a scale update as a simple squash animation.
      (Transformation|SetActorScale3D (Math|Vector|MakeVector (Math|Float|Lerp 1.0 0.5 _scaleanimation) 0.0 (Math|Float|Lerp 1.0 0.5 _scaleanimation))))
    (:Finished
      ;[0 0 0] Track the current side the player is on.
      (Variables|Default|SetbOnRightWall (not (Variables|Default|GetbOnRightWall)))
      ;[0 0 0] Reset bMoving so that the player is able to jump again.
      (Variables|Default|SetbMoving false))))

(event EventBeginPlay
  (|CallParentFunction)
  ;[0 0 0] Default initial starting side to the right.
  (Variables|Default|SetbOnRightWall true)
  ;[0 0 0] Store start location for use when calling the move functions
  (Variables|Default|SetStartLocation (Transformation|GetActorLocation)))

(event Input|ActionEvents|InputActionTouchAction
  (params (Key :type Key%20Structure))
  (:Pressed
    ;[0 0 0] Play sound effect
    (Audio|PlaySoundatLocation "/Game/EndlessRunnerCreator/CommonAssets/Audio/Whoosh_Cue_Audio.Whoosh_Cue_Audio" (Transformation|GetActorLocation) "0, 0, 0" 1.0 1.0 0.0 0 0 0)
    ;[0 0 0] Check if we can move and set moving to TRUE if we can.
    (if (CallFunction|CanMove)
      (Variables|Default|SetbMoving true)
      ;[0 0 0] Check which side the player is on and move to the other side.
      (if (Variables|Default|GetbOnRightWall)
        (CallFunction|MoveLeft)
        (else
          (CallFunction|MoveRight))))))

(fn ConstructionScript
  (|CallParentFunction))