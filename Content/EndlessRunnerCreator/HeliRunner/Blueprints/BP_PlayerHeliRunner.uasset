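; Player pawn for the HeliRunner endless runner mode, flown by holding a touch or mouse press to thrust upward and releasing to fall.
; While pressed, Tick adds upward acceleration to the physics collider and tilts the actor according to its vertical velocity.
; Pressing also boosts the Niagara trail and activates thruster audio.
; Physics stays disabled until LevelStarted, so the player does not fall during pause or start delay.
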(event EventBeginPlay
  (|CallParentFunction))

(event EventTick
  (params (DeltaSeconds :type Float%20%28single-precision%29))
  (bind _returnvalue (Transformation|GetVelocity))
  (if (and (CallFunction|CanMove) (Utilities|IsValid self))
    ;[0 0 0] Set actor rotation based on velocity to point in the direction the player is moving.
    (Transformation|SetActorRotation (Math|Rotator|MakeRotator (* (.z _returnvalue) (Variables|Default|GetRollRotationSpeed)) (* (.z _returnvalue) (Variables|Default|GetYawRotationSpeed)) 0.0) true)
    ;[0 0 0] Toggled when user touches the screen or mouse.
    (if (Variables|Default|GetbTouched)
      ;[0 0 0] Add Force vertically
      (Physics|AddForce (Variables|Default|GetCharacterCollider) "0, 0,2000.000000" "None" true))))

(event Input|ActionEvents|InputActionTouchAction
  (params (Key :type Key%20Structure :default "None"))
  ;[0 0 0] Touch screen and Desktop Input.
  (:Pressed
    (if (CallFunction|CanMove)
      ;[0 0 0] Toggle bTouched to be used on EventTick
      (Variables|Default|SetbTouched true)
      ;[0 0 0] Visual effect for the  particle trail to increase/decrease the scale to simulate a thruster effect
      (Niagara|SetNiagaraVariable(Float) (Variables|Default|GetNiagaraTrail) "SizeMult" 3.0)
      (Niagara|SetNiagaraVariable(Float) (Variables|Default|GetNiagaraTrail) "ForceMult" 1.5)
      ;[0 0 0] Play thruster audio component when pressed and disable it when released
      (Components|Activation|SetActive (Variables|Default|GetAudio) true false)))
  (:Released
    (if (CallFunction|CanMove)
      (Variables|Default|SetbTouched false)
      (Niagara|SetNiagaraVariable(Float) (Variables|Default|GetNiagaraTrail) "SizeMult" 1.0)
      (Niagara|SetNiagaraVariable(Float) (Variables|Default|GetNiagaraTrail) "ForceMult" 1.0)
      (Components|Activation|SetActive (Variables|Default|GetAudio) false true))))

(fn ConstructionScript
  (|CallParentFunction))

(fn LevelStarted
  (|CallParentFunction)
  ;[0 0 0] Physics starts disabled to stop the player falling whilst paused or during level start delay. Enable physics here when the game begins.
  (Physics|SetSimulatePhysics (Variables|Default|GetCharacterCollider) true))