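; Base obstacle Blueprint for the Voxel Runner endless runner game, extending a parent class's enable logic.
; EnableObject calls the parent, then plays a timeline that scales the actor from zero to full size so it appears to fly into view.
; It then calls random rotation and random location functions, which are empty here, apparently as hooks for child obstacles to override.
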(event Custom|AnimateScale
  ;[0 0 0] Visual animation to make it look like the object is flying into view rather than just appearing.
  (bind _scaleanimation (Timeline|ScaleAnim PlayFromStart)
    (:Update
      (Transformation|SetActorScale3D (Math|Vector|Lerp(Vector) "0, 0, 0" "1.000000,1.000000,1.000000" _scaleanimation)))))

(event EventTick
  (params (DeltaSeconds :type Float%20%28single-precision%29))
  (|CallParentFunction DeltaSeconds))

(fn ConstructionScript
  (|CallParentFunction))

(fn EnableObject
  (|CallParentFunction)
  (CallFunction|AnimateScale)
  (CallFunction|SetActorRandomRotation)
  (CallFunction|SetActorRandomLocation))

(fn SetActorRandomRotation)

(fn SetActorRandomLocation)