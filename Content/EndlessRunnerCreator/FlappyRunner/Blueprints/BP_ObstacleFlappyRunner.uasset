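; Flappy Runner pipe obstacle level piece that carries its own nested pickup and score checker, with enable/disable overrides for recycling.
; On BeginPlay it spawns a random class from the Pickups array, attaches it and starts it disabled, replacing a separate spawner.
; Each enable randomly decides whether to activate the pickup and re-arms the child-actor score checker against repeat triggering.
; Disabling the obstacle also disables its pickup.
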(event EventBeginPlay
  (|CallParentFunction)
  ;[0 0 0] This Game Type uses a nested pickup rather than a Spawner class
  ;;[1 1 1] Create Nested Pickup class, Attach it to this LevelPiece actor and call the disable interface to ensure that Pipes don't always start with the pickup enabled.
  (bind _returnvalue (Game|SpawnActorfromClass (CallFunction|GetRandomPickup) (Math|Transform|MakeTransform "0, 0, 0" "0, 0, 0" "1,1,1") "AlwaysSpawn" 0 true false 0))
  (Variables|Default|SetNestedPickupRef _returnvalue)
  (Transformation|AttachActorToActor (Variables|Default|GetNestedPickupRef) self "None" "KeepRelative" "KeepRelative" "KeepRelative" true)
  (Default|CallDisableObject (Variables|Default|GetNestedPickupRef)))

(fn ConstructionScript
  (|CallParentFunction))

(fn CheckShouldEnablePickup
  ;[0 0 0] Random chance that a pickup on this level piece will be enabled.
  (if (>= (Math|Random|RandomFloatinRange 0.0 1.0) 0.7)
    (Default|CallEnableObject (Variables|Default|GetNestedPickupRef))))

(fn EnableObject
  (|CallParentFunction)
  ;[0 0 0] Check for a random chance whrther the nested coin pickup should be activated when this obstacle is placed/recycled
  (CallFunction|CheckShouldEnablePickup)
  ;[0 0 0] Reset the ScoreChecker. This is included to avoid the player being able to activate the same nested score checker more than once.
  (Class|BPIPoolableObject|CallEnableObject(Message) (Variables|/Script/Engine.ChildActorComponent|GetChildActor (Variables|Default|GetScoreCheckActor))))

(fn DisableObject
  (|CallParentFunction)
  (Default|CallDisableObject (Variables|Default|GetNestedPickupRef)))

(fn GetRandomPickup
  (bind _pickups (Variables|Default|GetPickups))
  (return (Utilities|Array|Get(acopy) _pickups (Math|Random|RandomIntegerinRange 0 (- (Utilities|Array|Length _pickups) 1)))))