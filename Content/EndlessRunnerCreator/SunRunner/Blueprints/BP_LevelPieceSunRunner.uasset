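; BP_LevelPieceSunRunner is a level piece Blueprint for the SunRunner endless runner, scattering randomised grass across its surface.
; Its construction script runs the parent's script, then adds a set number of instances to an instanced static mesh component.
; Each instance gets a random X/Y position within a square area and a random uniform scale.
; BeginPlay only calls the parent, and Tick is disabled.
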(event EventBeginPlay
  (|CallParentFunction))

(event EventTick
  (params (DeltaSeconds :type Float%20%28single-precision%29))
  (|CallParentFunction DeltaSeconds) ; This node is disabled and will not be called.\nDrag off pins to build functionality.
)

(fn ConstructionScript
  (|CallParentFunction)
  ;[0 0 0] Create a specified number of instanced static meshes for the grass to add some randomisation.
  (for _index (range 0 (Variables|Default|GetInstancesToSpawn))
    (Components|InstancedStaticMesh|AddInstance (Variables|Default|GetInstancedStaticMesh) (Math|Transform|MakeTransform (Math|Vector|MakeVector (Math|Random|RandomFloatinRange -1.4e+03 1.4e+03) (Math|Random|RandomFloatinRange -1.4e+03 1.4e+03) 0.0) "0, 0, 0" (* "1.000000,1.000000,1.000000" (Math|Random|RandomFloatinRange 0.5 1.5))))))