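; Base game mode for the endless runner that persists the player's total currency and high score through a BP_Save slot.
; BeginPlay loads the existing save or creates one if none exists, and EndPlay writes a fresh save object with the current values.
; The Call functions for score, lives, currency, game state, pause, death and manager references are stubs that only return defaults.
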(event EventBeginPlay
  ;[0 0 0] Check for any save data to load.
  (CallFunction|LoadData))

(event EventEndPlay
  (params (EndPlayReason :type EEndPlayReason%20Enum :default "Destroyed"))
  ;[0 0 0] Make sure we save any progress when the game is ended in any manner
  (CallFunction|SaveData))

(fn ConstructionScript)

(fn LoadData
  ;[0 0 0] Check for existing saves.
  (bind _returnvalue (SaveGame|DoesSaveGameExist (Variables|Default|GetSaveDataName)))
  (if _returnvalue
    ;[0 0 0] If there is a save then load that and update the current variables to be tracked in game.
    (bind _returnvalue_2 (SaveGame|LoadGamefromSlot (Variables|Default|GetSaveDataName)))
    (bind _asbp_save (Utilities|Casting|CastToBP_Save _returnvalue_2))
    (bind _output_get (Variables|Default|SetSaveRef _asbp_save))
    (Variables|Ints|SetTotalCurrency (Variables|/Game/EndlessRunnerCreator/CommonAssets/Blueprints/Game/BP_Save.BP_Save_C|GetCoins _output_get))
    (Variables|Ints|SetHighScore (Variables|/Game/EndlessRunnerCreator/CommonAssets/Blueprints/Game/BP_Save.BP_Save_C|GetHighScore (Variables|Default|GetSaveRef)))
    (else
      ;[0 0 0] If there's no save then create one.
      (CallFunction|SaveData))))

(fn SaveData
  ;[0 0 0] Create a save, pass the tracked variables and assign it to the given save slot.
  (bind _returnvalue (SaveGame|CreateSaveGameObject "/Game/EndlessRunnerCreator/CommonAssets/Blueprints/Game/BP_Save.BP_Save_C"))
  (bind _output_get (Variables|Default|SetSaveRef _returnvalue))
  (Variables|/Game/EndlessRunnerCreator/CommonAssets/Blueprints/Game/BP_Save.BP_Save_C|SetCoins _output_get (Variables|Ints|GetTotalCurrency))
  (Variables|/Game/EndlessRunnerCreator/CommonAssets/Blueprints/Game/BP_Save.BP_Save_C|SetHighScore (Variables|Default|GetSaveRef) (Variables|Ints|GetHighScore))
  (SaveGame|SaveGametoSlot (Variables|Default|GetSaveRef) (Variables|Default|GetSaveDataName)))

(fn CallAddCurrency
  (params (CurrencyToAdd :type Integer))
  (return false))

(fn CallAddLife
  (params (LivesToAdd :type Integer))
  (return false))

(fn CallGetCurrentGameState
  (return "NewEnumerator0"))

(fn CallGetScore
  (return 0))

(fn CallPausePressed
  (return false))

(fn CallPlayerDied
  (params (PlayerRef :type Actor%20Object%20Reference))
  (return false))

(fn CallSetGameState
  (params (CurrentState :type EGameState%20Enum :default "NewEnumerator0"))
  (return false))

(fn CallSetLevelHUDRef
  (params (LevelHUD :type WBP%20HUD%20Base%20Object%20Reference))
  (return false))

(fn CallSetLevelManager
  (params (LevelManager :type BP%20Level%20Manager%20Base%20Object%20Reference))
  (return false))

(fn CallSetMaxLives
  (params (Lives :type Integer))
  (return false))

(fn CallSetRespawnDelay
  (params (RespawnDelay :type Float%20%28single-precision%29))
  (return false))

(fn CallSetScore
  (params (Score :type Integer))
  (return false))