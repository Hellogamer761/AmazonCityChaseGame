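; 2D player Blueprint for the Lizard Runner endless runner, extending a parent player class with Paper2D flipbook animation.
; BeginPlay caches the starting flipbook as the default.
; The jump and land effect events call their parent versions, play the matching flipbook, then restore the default after a delay equal to that flipbook's length.
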(event EventBeginPlay
  (|CallParentFunction)
  ;[0 0 0] Set the default flipbook animation
  (Variables|Default|SetFB_Default (Class|PaperFlipbookComponent|GetFlipbook (Variables|Default|GetPaperFlipbook))))

(event EventJumpEffect
  (bind _paperflipbook (Variables|Default|GetPaperFlipbook))
  (|CallParentFunction)
  ;[0 0 0] Play jump flipbook animation and then return to the default animation at the end of the jump flipbook.
  (Sprite|SetFlipbook _paperflipbook (Variables|Default|GetFB_Jump))
  (Utilities|FlowControl|Delay (Class|PaperFlipbookComponent|GetFlipbookLength _paperflipbook))
  (Sprite|SetFlipbook (Variables|Default|GetPaperFlipbook) (Variables|Default|GetFB_Default)))

(event EventLandEffect
  (|CallParentFunction)
  ;[0 0 0] Play land flipbook animation and then return to the default animation at the end of the land flipbook.
  (Sprite|SetFlipbook (Variables|Default|GetPaperFlipbook) (Variables|Default|GetFB_Land))
  (Utilities|FlowControl|Delay (Class|PaperFlipbookComponent|GetFlipbookLength (Variables|Default|GetPaperFlipbook)))
  (Sprite|SetFlipbook (Variables|Default|GetPaperFlipbook) (Variables|Default|GetFB_Default)))

(fn ConstructionScript
  (|CallParentFunction))