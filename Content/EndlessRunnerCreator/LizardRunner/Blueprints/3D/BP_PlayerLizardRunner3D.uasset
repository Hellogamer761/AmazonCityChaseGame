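; Player Blueprint for the 3D Lizard Runner game in EndlessRunnerCreator, adding skeletal animation to jumping and landing.
; It extends the parent's JumpEffect and LandEffect events, calling the parent logic first and then playing the matching jump or land montage on the SkeletalMesh.
; BeginPlay and the construction script only forward to the parent, so any other player behavior is inherited.
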(event EventBeginPlay
  (|CallParentFunction))

(event EventJumpEffect
  (|CallParentFunction)
  ;[0 0 0] Play jump animation montage
  (Animation|Montage|PlayMontage (Variables|Default|GetSkeletalMesh) "/Game/EndlessRunnerCreator/CommonAssets/Animations/SK_Player_Anim_PlayerSkeleton_Jump_Montage.SK_Player_Anim_PlayerSkeleton_Jump_Montage" 1.0 0.0 "Default"))

(event EventLandEffect
  (|CallParentFunction)
  ;[0 0 0] Play land animation montage
  (Animation|Montage|PlayMontage (Variables|Default|GetSkeletalMesh) "/Game/EndlessRunnerCreator/CommonAssets/Animations/SK_Player_Anim_PlayerSkeleton_Land_Montage.SK_Player_Anim_PlayerSkeleton_Land_Montage" 1.0 0.0 "Default"))

(fn ConstructionScript
  (|CallParentFunction))